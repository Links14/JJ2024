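; First-person player character with a battery-limited flashlight and a gory death on contact with a Monster.
; Enhanced Input drives look, movement, hold-to-crouch and a hold-to-use flashlight, whose charge Tick drains and prints for debugging.
; KillPlayer disables input, swaps to a ragdolled headless mesh, releases camera control and launches a physics Sphere as the severed head.
; Blood decals mark the death spot and the Sphere's hard impacts and resting point.
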(event OnComponentHit(Sphere)
  (params (HitComponent :type Primitive%20Component%20Object%20Reference) (OtherActor :type Actor%20Object%20Reference) (OtherComp :type Primitive%20Component%20Object%20Reference) (NormalImpulse :type Vector :default "0, 0, 0") (Hit :type Hit%20Result%20Structure%20%28by%20ref%29))
  (bind (_bblockinghit _binitialoverlap _time _distance _location _impactpoint _normal) (Collision|BreakHitResult Hit))
  (if (> (Math|Vector|VectorLength NormalImpulse) 3e+03)
    (Rendering|Decal|SpawnDecalatLocation "/Game/Materials-PostProcessing/Decals/Blood.Blood" "1.000000,50.000000,50.000000" _location (Math|Rotator|MakeRotfromX _normal) 0.0)
    (Audio|PlaySound2D "/Game/Sounds/BloodSplat.BloodSplat" 1.0 1.0 0.0 0 0)))

(event OnComponentSleep(Sphere)
  (params (SleepingComponent :type Primitive%20Component%20Object%20Reference) (BoneName :type Name :default "None"))
  (bind _returnvalue (Transformation|GetWorldLocation SleepingComponent))
  (bind (_x _y _z) (Math|Vector|BreakVector _returnvalue))
  (bind _outhit (Collision|LineTraceByChannel _returnvalue (Math|Vector|MakeVector _x _y (- _z 2e+01)) "TraceTypeQuery1" false 0 "None"))
  (Rendering|Decal|SpawnDecalatLocation "/Game/Materials-PostProcessing/Decals/Blood.Blood" "1.000000,50.000000,50.000000" (.location _outhit) "-90.000000,0.000000,0.000000" 0.0)
  (Audio|PlaySound2D "/Game/Sounds/BloodSplat.BloodSplat" 1.0 1.0 0.0 0 0))

(event Input|EnhancedActionEvents|EnhancedInputActionIA_Crouch
  (params (ActionValue :type Boolean) (ElapsedSeconds :type Float%20%28double-precision%29) (TriggeredSeconds :type Float%20%28double-precision%29) (InputAction :type Input%20Action%20Object%20Reference :default "/Game/Blueprints/Player/Input/IA_Crouch.IA_Crouch"))
  ;[1 1 1] Crouch
  (:Triggered
    (Character|Crouch))
  (:Canceled
    (Character|UnCrouch :!label _label))
  (:Completed
    (goto _label)))

(event Input|EnhancedActionEvents|EnhancedInputActionIA_Flashlight
  (params (ActionValue :type Boolean) (ElapsedSeconds :type Float%20%28double-precision%29) (TriggeredSeconds :type Float%20%28double-precision%29) (InputAction :type Input%20Action%20Object%20Reference :default "/Game/Blueprints/Player/Input/IA_Flashlight.IA_Flashlight"))
  (bind _spotlight (Variables|Default|GetSpotLight))
  (bind _flashlight (Variables|Default|GetFlashlight))
  (bind _returnvalue (> _flashlight 0.0))
  ;[1 1 1] Flashlight
  (:Triggered
    (Rendering|SetVisibility _spotlight _returnvalue false))
  (:Started
    (if _returnvalue :!label _label
      (Audio|PlaySound2D "/Game/Sounds/FlashlightToggle.FlashlightToggle" 1.0 1.0 0.0 0 0)))
  (:Canceled
    (Rendering|SetVisibility _spotlight false false :!label _label_2)
    (goto _label))
  (:Completed
    (goto _label_2)))

(event Input|EnhancedActionEvents|EnhancedInputActionIA_Move
  (params (ActionValue :type Vector%202D%20Structure) (ElapsedSeconds :type Float%20%28double-precision%29) (TriggeredSeconds :type Float%20%28double-precision%29) (InputAction :type Input%20Action%20Object%20Reference :default "/Game/Blueprints/Player/Input/IA_Move.IA_Move"))
  (bind _returnvalue (Pawn|GetControlRotation :!class /Script/Engine.Pawn))
  ;[1 1 1] Movement
  (Pawn|Input|AddMovementInput (Math|Vector|GetRightVector (Math|Rotator|MakeRotator (.roll _returnvalue) 0.0 (.yaw _returnvalue))) (.x ActionValue) false)
  (Pawn|Input|AddMovementInput (Math|Vector|GetForwardVector (Math|Rotator|MakeRotator 0.0 0.0 (.yaw _returnvalue))) (.y ActionValue) false))

(event Input|EnhancedActionEvents|EnhancedInputActionIA_Look
  (params (ActionValue :type Vector%202D%20Structure) (ElapsedSeconds :type Float%20%28double-precision%29) (TriggeredSeconds :type Float%20%28double-precision%29) (InputAction :type Input%20Action%20Object%20Reference :default "/Game/Blueprints/Player/Input/IA_Look.IA_Look"))
  ;[1 1 1] Camera
  (Pawn|Input|AddControllerYawInput (.x ActionValue))
  (Pawn|Input|AddControllerPitchInput (.y ActionValue)))

(event EventBeginPlay
  (bind _asplayer_controller (Utilities|Casting|CastToPlayerController (Pawn|GetController)))
  (Utilities|IsValid (PlayerController|LocalPlayerSubsystems|GetEnhancedInputLocalPlayerSubsystem _asplayer_controller)
    (:Is%20Valid
      (Input|AddMappingContext (PlayerController|LocalPlayerSubsystems|GetEnhancedInputLocalPlayerSubsystem _asplayer_controller) "/Game/Blueprints/Player/MappingContext.MappingContext" 0 "(bIgnoreAllPressedKeysUntilRelease=True,bForceImmediately=False,bNotifyUserSettings=False)"))))

(event EventTick
  (params (DeltaSeconds :type Float%20%28single-precision%29))
  (Development|PrintString (Utilities|String|ToString(Float) (Variables|Default|GetFlashlight)))
  (if (and (Input|EnhancedActionValues|GetIA_Flashlight) (> (Variables|Default|GetFlashlight) 0.0))
    (Variables|Default|SetFlashlight (- (Variables|Default|GetFlashlight) DeltaSeconds))
    (if (not (> (Variables|Default|GetFlashlight) 0.0)) ; Flashlight dies
      ;[1 1 1] Flashlight
      (Rendering|SetVisibility (Variables|Default|GetSpotLight) false false)
      (if (> (Variables|Default|GetFlashlight) 0.0)
        (Audio|PlaySound2D "/Game/Sounds/FlashlightToggle.FlashlightToggle" 1.0 1.0 0.0 0 0)))))

(event Collision|EventHit
  (params (MyComp :type Primitive%20Component%20Object%20Reference) (Other :type Actor%20Object%20Reference) (OtherComp :type Primitive%20Component%20Object%20Reference) (bSelfMoved :type Boolean) (HitLocation :type Vector :default "0, 0, 0") (HitNormal :type Vector :default "0, 0, 0") (NormalImpulse :type Vector :default "0, 0, 0") (Hit :type Hit%20Result%20Structure%20%28by%20ref%29))
  (Utilities|Casting|CastToMonster Other)
  (CallFunction|KillPlayer))

(fn ConstructionScript)

(fn KillPlayer
  (bind _returnvalue (Transformation|GetActorLocation))
  (bind _sphere (Variables|Default|GetSphere))
  (bind _camera (Variables|Default|GetCamera))
  (bind _mesh (Variables|Character|GetMesh))
  (bind (_x _y _z) (Math|Vector|BreakVector _returnvalue))
  (if (not (Variables|Default|GetDead))
    (Variables|Default|SetDead true)
    (Input|DisableInput (Game|GetPlayerController 0))
    (Collision|SetCollisionEnabled (Variables|Collision|GetCapsuleComponent) "NoCollision")
    (Collision|SetCollisionEnabled _sphere "PhysicsOnly")
    (Physics|SetSimulatePhysics _sphere true)
    (Variables|/Script/Engine.CameraComponent|SetbUsePawnControlRotation _camera false)
    (Physics|AddForce _sphere (* (Math|Vector|GetForwardVector _camera) "-30000.000000,-30000.000000,-30000.000000") "None" true)
    (Variables|/Script/Engine.SkeletalMeshComponent|SetSkeletalMeshAsset _mesh "/Game/Blueprints/Player/Model/HumanHeadless.HumanHeadless")
    (Class|PrimitiveComponent|SetOwnerNoSee _mesh false)
    (Physics|SetSimulatePhysics _mesh true)
    (bind _outhit (Collision|LineTraceByChannel _returnvalue (Math|Vector|MakeVector _x _y (- _z 1e+02)) "TraceTypeQuery1" false 0 "None"))
    (if (.bblockinghit _outhit)
      (Rendering|Decal|SpawnDecalatLocation "/Game/Materials-PostProcessing/Decals/Blood.Blood" "1.000000,200.000000,200.000000" (.location _outhit) "-90.000000,0.000000,0.000000" 0.0))
    (Audio|PlaySoundatLocation "/Engine/VREditor/Sounds/UI/Invalid_Action.Invalid_Action" (Transformation|GetActorLocation) "0, 0, 0" 1.0 1.0 0.0 0 0 0 0)))